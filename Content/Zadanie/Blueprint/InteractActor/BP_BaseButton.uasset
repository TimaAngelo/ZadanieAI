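; Base interactable button actor that activates all AI characters in the level when interacted with.
; Its collision box registers the button in the overlapping BP_ThirdPersonCharacter's Button variable and clears it when the overlap ends.
; Interact finds every MyBaseAICharacter and sets the IsActivated key to true on its blackboard.
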(event `/Game/Zadanie/Blueprint/Interface/BP_InteractInterface.Interact`
  (bind _outactors (`GameplayStatics.GetAllActorsOfClass` "/Game/Zadanie/Blueprint/AI/BaseAI/MyBaseAICharacter.MyBaseAICharacter_C"))
  (for _array_element _outactors
    (`BlackboardComponent.SetValueAsBool` (`AIBlueprintHelperLibrary.GetBlackboard` _array_element) "IsActivated" true)))

(event `self.CollisionBox.OnComponentBeginOverlap`
  (params (OverlappedComponent :type "PrimitiveComponent Object Reference") (OtherActor :type "Actor Object Reference") (OtherComp :type "PrimitiveComponent Object Reference") (OtherBodyIndex :type Integer) (bFromSweep :type Boolean) (SweepResult :type "HitResult Structure (by ref)"))
  (bind _asbp_third_person_character (cast `/Game/Zadanie/Blueprint/Character/BP_ThirdPersonCharacter` OtherActor))
  (set `/Game/Zadanie/Blueprint/Character/BP_ThirdPersonCharacter.Button` self _asbp_third_person_character))

(event `self.CollisionBox.OnComponentEndOverlap`
  (params (OverlappedComponent :type "PrimitiveComponent Object Reference") (OtherActor :type "Actor Object Reference") (OtherComp :type "PrimitiveComponent Object Reference") (OtherBodyIndex :type Integer))
  (bind _asbp_third_person_character (cast `/Game/Zadanie/Blueprint/Character/BP_ThirdPersonCharacter` OtherActor))
  (set `/Game/Zadanie/Blueprint/Character/BP_ThirdPersonCharacter.Button` null _asbp_third_person_character))

(fn `UserConstructionScript`)